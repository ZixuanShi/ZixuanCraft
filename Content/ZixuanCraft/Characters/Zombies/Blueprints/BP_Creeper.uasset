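; BP_Creeper is a creeper enemy, filed under zombie characters, that attacks by exploding.
; When its Aggressive component fires OnAttack, a sphere overlap sized by AttackRange gathers nearby WorldDynamic and Pawn actors.
; Each receives the component's Damage with the AI controller as instigator, with the intent of also destroying nearby blocks.
; The creeper then spawns an explosion particle effect at its location and destroys itself.
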(event `self.Aggressive.OnAttack`
  (params (TargetActor :type "Actor Object Reference"))
  ;[1 1 1] Apply AOE damage to all the actors around this creeper, should destroy blocks nearby
  (bind _outactors (`KismetSystemLibrary.SphereOverlapActors` (`self.K2_GetActorLocation`) (`AggressiveComponent.AttackRange` (`self.Aggressive`)) (`|MakeArray` "ObjectTypeQuery2" "ObjectTypeQuery3" :!type "EObjectTypeQuery Enum") "/Script/Engine.Actor"))
  (for _array_element _outactors
    (`GameplayStatics.ApplyDamage` _array_element (`AggressiveComponent.Damage` (`self.Aggressive`)) (`AIBlueprintHelperLibrary.GetAIController` null) self "/Script/Engine.DamageType"))
  (`GameplayStatics.SpawnEmitterAtLocation` "/Game/ZixuanCraft/Common/Particles/P_Explosion.P_Explosion" (`self.K2_GetActorLocation`))
  (`self.K2_DestroyActor`))

(fn `UserConstructionScript`)