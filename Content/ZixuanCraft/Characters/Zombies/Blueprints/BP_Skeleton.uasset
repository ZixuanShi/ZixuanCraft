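; BP_Skeleton is a zombie-category skeleton character that attacks at range by firing projectiles at its target.
; When its Aggressive component fires OnAttack, it spawns BP_FirstPersonProjectile slightly ahead of the GunMesh "Ammo" socket, rotated to face the target's location.
; The skeleton is set as owner and instigator, and the projectile takes its damage value from the Aggressive component.
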(event `self.Aggressive.OnAttack`
  (params (TargetActor :type "Actor Object Reference"))
  (bind _returnvalue (`self.K2_GetActorLocation` TargetActor))
  (bind _returnvalue_2 (`SceneComponent.GetSocketLocation` (`self.GunMesh`) "Ammo"))
  (bind _returnvalue_3 (+ _returnvalue_2 (* (`KismetMathLibrary.GetDirectionUnitVector` _returnvalue_2 _returnvalue) 10.0)))
  ;[1 1 1] Shoot a projectile towards target
  (bind _returnvalue_4 (`|SpawnActorFromClass` "/Game/ZixuanCraft/GameObjects/Weapons/BP_FirstPersonProjectile.BP_FirstPersonProjectile_C" (`KismetMathLibrary.MakeTransform` _returnvalue_3 (`KismetMathLibrary.FindLookAtRotation` _returnvalue_3 _returnvalue)) "Undefined" "OverrideRootScale" self self))
  (set `ZixuanCraftProjectile.Damage` (`AggressiveComponent.Damage` (`self.Aggressive`)) _returnvalue_4))

(fn `UserConstructionScript`)