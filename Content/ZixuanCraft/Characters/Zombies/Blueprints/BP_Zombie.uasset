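; BP_Zombie is a zombie NPC Blueprint that damages its target when it attacks.
; The OnAttack event from its Aggressive member applies that member's damage value to the target, with the zombie's controller as instigator.
; It then sets the Attacking flag on the anim instance, and a short one-shot timer clears it on Zombie_AnimBP.
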(event `self.Aggressive.OnAttack`
  (params (TargetActor :type "Actor Object Reference"))
  ;[1 1 1] Apply damage to the target
  (`GameplayStatics.ApplyDamage` TargetActor (`AggressiveComponent.Damage` (`self.Aggressive`)) (`self.GetController`) self "/Script/Engine.DamageType")
  (set `NPCAnimInstance.bAttacking` true (`self.GetNPCAnimInstance`))
  (`KismetSystemLibrary.K2_SetTimerDelegate` (delegate `ResetAttackAnimation`) 0.5))

(event `ResetAttackAnimation`
  ;[1 1 1] Apply damage to the target
  (bind _aszombie_anim_bp (cast `/Game/ZixuanCraft/Characters/Zombies/Animations/Zombie_AnimBP` (`SkeletalMeshComponent.GetAnimInstance` (`self.Mesh`))))
  (set `NPCAnimInstance.bAttacking` false _aszombie_anim_bp))

(fn `UserConstructionScript`)