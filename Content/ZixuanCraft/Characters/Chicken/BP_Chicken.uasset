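; BP_Chicken is a damageable chicken character that drops loot when killed.
; On any damage it subtracts health; a surviving chicken switches its agent state to Engaged and plays a hit sound, throttled to the sound's duration.
; When health falls below zero it flags death in its anim blueprint, waits out the death lifespan, spawns BP_ChickenLoot with a roasted chicken icon and destroys itself.
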(event `self.ReceiveAnyDamage`
  (params (Damage :type "Float (single-precision)") (DamageType :type "DamageType Object Reference") (InstigatedBy :type "Controller Object Reference") (DamageCauser :type "Actor Object Reference"))
  ;[1 1 1] Substract Health
  (bind _output_get (set `self.Health` (- (`self.Health`) Damage)))
  ;[1 1 1] Check if dead
  (if (< _output_get 0.0)
    (set `self.AgentState` "Dead")
    ;[1 1 1] Play death animation
    (bind _aschicken_anim_bp (cast `/Game/ZixuanCraft/Characters/Chicken/Animations/Chicken_AnimBP` (`SkeletalMeshComponent.GetAnimInstance` (`self.Mesh`))))
    (set `/Game/ZixuanCraft/Characters/Chicken/Animations/Chicken_AnimBP.IsDead` true _aschicken_anim_bp)
    ;[1 1 1] Wait for a few seconds for the animation, set a timer
    (`KismetSystemLibrary.Delay` (`self.DeathLifeSpan`))
    (`|SpawnActorFromClass` "/Game/ZixuanCraft/Characters/Chicken/BP_ChickenLoot.BP_ChickenLoot_C" (`KismetMathLibrary.MakeTransform` (`self.K2_GetActorLocation`) (`self.K2_GetActorRotation`)) "Undefined" "OverrideRootScale" null true null "/Game/ZixuanCraft/Characters/Chicken/Textures/T_RoastedChickenThumbnail.T_RoastedChickenThumbnail")
    (`self.K2_DestroyActor`)
    (else
      (set `self.AgentState` "Engaged")
      ;[1 1 1] Play on hit sound
      (if (`self.bCanPlaySound`)
        (`GameplayStatics.PlaySoundAtLocation` (`self.ChickenSound`) (`self.K2_GetActorLocation`) (struct) 1.0 1.0 0.0 null null null)
        ;[1 1 1] Delayed set play sound timer
        (set `self.bCanPlaySound` false)
        (`KismetSystemLibrary.Delay` (`SoundBase.Duration` (`self.ChickenSound`)))
        (set `self.bCanPlaySound` true)))))

(fn `UserConstructionScript`)