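; BP_VoxelDebugger is a debug actor that spawns a 3D grid of BP_DebugCube actors to visualize voxel indexing.
; On BeginPlay, nested XYZ loops place cubes at CubeLength spacing, passing each its grid coordinate and flattened index.
; GetIndex maps coordinates to slots in the pre-sized AllCubes array.
; UpdateMesh only prints a hit location and its GetIndexFromLocation result; its cube-destroy logic is disconnected.
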(event `self.ReceiveBeginPlay`
  (bind (_xyzindices_x _xyzindices_y _xyzindices_z) (break `IntVector` (`self.XYZIndices`)))
  (bind (_xyzindices_x_2 _xyzindices_y_2 _xyzindices_z_2) (break `IntVector` (`self.XYZIndices`)))
  (`KismetArrayLibrary.Array_Resize` (`self.AllCubes`) (* (`self.CubeCountXYSquared`) (`self.CubeCountZ`)))
  ;[1 1 1] X
  (for _index (range (`self.CubeCountXY`))
    ;[1 1 1] Y
    (for _index_2 (range (`self.CubeCountXY`))
      ;[1 1 1] Z
      (for _index_3 (range (`self.CubeCountZ`))
        (bind _intvector (make `IntVector` _index _index_2 _index_3))
        (set `self.XYZIndices` _intvector)
        (bind _returnvalue (`KismetMathLibrary.Conv_IntVectorToVector` _intvector))
        (bind _returnvalue_2 (`|SpawnActorFromClass` "/Game/ZixuanCraft/Debug/BP_DebugCube.BP_DebugCube_C" (`KismetMathLibrary.MakeTransform` (* _returnvalue (`self.CubeLength`))) "Undefined" "OverrideRootScale" null _returnvalue (`self.GetIndex` _xyzindices_x _xyzindices_y _xyzindices_z) null))
        (`KismetArrayLibrary.Array_Set` (`self.AllCubes`) (`self.GetIndex` _xyzindices_x_2 _xyzindices_y_2 _xyzindices_z_2) _returnvalue_2)))))

(fn `UpdateMesh`
  (params (HitLocation :type "Vector Structure"))
  (`KismetSystemLibrary.PrintString` (`KismetStringLibrary.Concat_StrStr` (`KismetStringLibrary.Conv_VectorToString` HitLocation) ", " (`KismetStringLibrary.Conv_IntToString` (`self.GetIndexFromLocation` HitLocation)))))

(fn `UserConstructionScript`)