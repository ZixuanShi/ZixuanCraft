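; BP_TerrainVoxel is a terrain voxel actor that populates the world with trees and creatures and cleans them up when it is removed.
; Its Spawn event places a BP_Tree for the Tree type, or randomly spawns a chicken or zombie with its behavior tree, raised above the location, for Spawnable.
; Everything spawned is tracked in SpawnedObjects, and the Destroyed event destroys any still-valid entries.
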(event `self.Spawn`
  (params (Type :type "ECubeType Enum" :default "Empty") (Location :type "Vector Structure"))
  (bind _returnvalue (+ Location (0.0 0.0 100.0)))
  (switch `ECubeType` Type
    (:`Tree`
      (bind _returnvalue_2 (`|SpawnActorFromClass` "/Game/ZixuanCraft/GameObjects/BP_Tree.BP_Tree_C" (`KismetMathLibrary.Conv_VectorToTransform` Location) "Undefined" "OverrideRootScale" null null))
      (`KismetArrayLibrary.Array_Add` (`self.SpawnedObjects`) _returnvalue_2))
    (:`Spawnable`
      (switch `int` (`KismetMathLibrary.RandomInteger` 2)
        (:`0`
          (bind _returnvalue_3 (`AIBlueprintHelperLibrary.SpawnAIFromClass` "/Game/ZixuanCraft/GameObjects/Spawnable/AI/Chicken/BP_Chicken.BP_Chicken_C" "/Game/ZixuanCraft/GameObjects/Spawnable/AI/Chicken/BT_Chicken.BT_Chicken" _returnvalue (struct) false null))
          (`KismetArrayLibrary.Array_Add` (`self.SpawnedObjects`) _returnvalue_3))
        (:`1`
          (bind _returnvalue_4 (`AIBlueprintHelperLibrary.SpawnAIFromClass` "/Game/ZixuanCraft/GameObjects/Spawnable/AI/Zombie/BP_Zombie.BP_Zombie_C" "/Game/ZixuanCraft/GameObjects/Spawnable/AI/Zombie/BT_Zombie.BT_Zombie" _returnvalue (struct) false null))
          (`KismetArrayLibrary.Array_Add` (`self.SpawnedObjects`) _returnvalue_4))))))

(event `self.ReceiveDestroyed`
  (for _array_element (`self.SpawnedObjects`)
    (`/Engine/EditorBlueprintResources/StandardMacros.IsValid` _array_element
      (:`Is Valid`
        (`self.K2_DestroyActor` _array_element)))))

(fn `UserConstructionScript`)