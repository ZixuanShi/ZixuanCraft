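; Voxel terrain actor that populates itself with NPCs and removes them when it is destroyed.
; SpawnNPC samples 2D simplex noise at the given location and uses the parity of the rounded value to pick a chicken or a zombie.
; The chosen AI spawns with its behavior tree slightly above that point and is tracked in SpawnedObjects.
; On Destroyed, every still-valid tracked actor is destroyed.
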(event `self.SpawnNPC`
  (params (Location :type "Vector Structure"))
  (bind _returnvalue (+ Location (0.0 0.0 100.0)))
  (bind _returnvalue_2 (`SimplexNoiseBPLibrary.SimplexNoise2D` (.x Location) (.y Location)))
  (switch `int` (mod (`KismetMathLibrary.Conv_Int64ToInt` (`KismetMathLibrary.Round64` _returnvalue_2)) 2)
    (:`0`
      (bind _returnvalue_3 (`AIBlueprintHelperLibrary.SpawnAIFromClass` "/Game/ZixuanCraft/Characters/Chicken/BP_Chicken.BP_Chicken_C" "/Game/ZixuanCraft/Characters/Chicken/AI/BT_Chicken.BT_Chicken" _returnvalue (struct) false null))
      (`KismetArrayLibrary.Array_Add` (`self.SpawnedObjects`) _returnvalue_3))
    (:`1`
      (bind _returnvalue_4 (`AIBlueprintHelperLibrary.SpawnAIFromClass` "/Game/ZixuanCraft/Characters/Zombie/BP_Zombie.BP_Zombie_C" "/Game/ZixuanCraft/Characters/Zombie/AI/BT_Zombie.BT_Zombie" _returnvalue (struct) false null))
      (`KismetArrayLibrary.Array_Add` (`self.SpawnedObjects`) _returnvalue_4))))

(event `self.ReceiveDestroyed`
  (for _array_element (`self.SpawnedObjects`)
    (`/Engine/EditorBlueprintResources/StandardMacros.IsValid` _array_element
      (:`Is Valid`
        (`self.K2_DestroyActor` _array_element)))))

(fn `UserConstructionScript`)