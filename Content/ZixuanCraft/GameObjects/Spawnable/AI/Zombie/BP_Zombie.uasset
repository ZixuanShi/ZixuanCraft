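; Zombie enemy character that takes damage, dies and melee-attacks a given target.
; Damage lowers Health and sets AgentState to Engaged, or to Dead below zero, crediting a FirstPersonCharacter killer before playing death animation and sound, disabling collision and setting a life span.
; Attack applies damage behind a timer-based cooldown.
; Attack and death animations are driven by flags on Zombie_AnimBP, with a timer clearing the attack flag.
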(event `self.ReceiveAnyDamage`
  (params (Damage :type "Float (single-precision)") (DamageType :type "DamageType Object Reference") (InstigatedBy :type "Controller Object Reference") (DamageCauser :type "Actor Object Reference"))
  ;[1 1 1] Substract Health
  (bind _output_get (set `self.Health` (- (`self.Health`) Damage)))
  ;[1 1 1] Check if dead
  (if (< _output_get 0.0)
    (set `self.AgentState` "Dead")
    ;[1 1 1] Increment player slained enemies count
    (bind _asfirst_person_character (cast `/Game/ZixuanCraft/GameObjects/FirstPerson/FirstPersonCharacter` DamageCauser))
    (`/Engine/EditorBlueprintResources/StandardMacros.IncrementInt` (`/Game/ZixuanCraft/GameObjects/FirstPerson/FirstPersonCharacter.SlainedEnemies` _asfirst_person_character)
      (:`  `
        ;[1 1 1] Play death animation
        (bind _aszombie_anim_bp (cast `/Game/ZixuanCraft/GameObjects/Spawnable/AI/Zombie/Animations/Zombie_AnimBP` (`SkeletalMeshComponent.GetAnimInstance` (`self.Mesh`))))
        (set `/Game/ZixuanCraft/GameObjects/Spawnable/AI/Zombie/Animations/Zombie_AnimBP.IsDead` true _aszombie_anim_bp)
        (`GameplayStatics.PlaySoundAtLocation` "/Game/ZixuanCraft/GameObjects/Spawnable/AI/Zombie/Audio/Minecraft_Zombie_Cue.Minecraft_Zombie_Cue" (`self.K2_GetActorLocation`) (struct) 1.0 1.0 0.0 null null null)
        ;[1 1 1] Set life span and disable collision
        (`self.SetLifeSpan` (`self.DeathLifeSpan`))
        (`PrimitiveComponent.SetCollisionEnabled` (`self.CapsuleComponent`) "NoCollision")
        (`PrimitiveComponent.SetCollisionEnabled` (`self.Mesh`) "NoCollision")))
    (else
      (set `self.AgentState` "Engaged"))))

(event `self.Attack`
  (params (Target :type "Actor Object Reference"))
  (if (`self.CanAttack`)
    (`GameplayStatics.ApplyDamage` Target (`self.Damage`) (`self.GetController`) self)
    (bind _aszombie_anim_bp (cast `/Game/ZixuanCraft/GameObjects/Spawnable/AI/Zombie/Animations/Zombie_AnimBP` (`SkeletalMeshComponent.GetAnimInstance` (`self.Mesh`))))
    (set `/Game/ZixuanCraft/GameObjects/Spawnable/AI/Zombie/Animations/Zombie_AnimBP.IsAttacking` true _aszombie_anim_bp)
    (`KismetSystemLibrary.K2_SetTimerDelegate` (delegate `CustomEvent_0`) 0.5)
    (set `self.CanAttack` false)
    (`KismetSystemLibrary.K2_SetTimerDelegate` (delegate `Set AttackCooldown`) (`self.AttackCooldown`))))

(event `CustomEvent_0`
  (bind _aszombie_anim_bp (cast `/Game/ZixuanCraft/GameObjects/Spawnable/AI/Zombie/Animations/Zombie_AnimBP` (`SkeletalMeshComponent.GetAnimInstance` (`self.Mesh`))))
  (set `/Game/ZixuanCraft/GameObjects/Spawnable/AI/Zombie/Animations/Zombie_AnimBP.IsAttacking` false _aszombie_anim_bp))

(event `Set AttackCooldown`
  (set `self.CanAttack` true))

(fn `UserConstructionScript`)