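; BP_Tree is a tree actor that varies its shape by randomly scaling its TreeTrunk and Leaves components on BeginPlay.
; The trunk varies only in height, while the leaves vary independently on all three axes within min/max variables.
; Relative Z offsets derived from those scales raise or lower the trunk and leaves to compensate for the size change.
; The construction script is empty, so variation appears only at runtime.
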(event `self.ReceiveBeginPlay`
  ;[1 1 1] Randomly set tree trunk height scale
  (bind _output_get (set `self.TrunkZ` (`KismetMathLibrary.RandomFloatInRange` (`self.TrunkZMin`) (`self.TrunkZMax`))))
  (`SceneComponent.SetRelativeScale3D` (`self.TreeTrunk`) (`KismetMathLibrary.MakeVector` 1.0 1.0 _output_get))
  ;[1 1 1] Tune height offset
  (`SceneComponent.K2_AddRelativeLocation` (`self.TreeTrunk`) (`KismetMathLibrary.MakeVector` 0.0 0.0 (* 50.0 (- (`self.TrunkZ`) 1.0))) false false)
  ;[1 1 1] Randomly set tree leaves width length height scale
  (set `self.LeavesX` (`KismetMathLibrary.RandomFloatInRange` (`self.LeavesXYMin`) (`self.LeavesXYMax`)))
  (set `self.LeavesY` (`KismetMathLibrary.RandomFloatInRange` (`self.LeavesXYMin`) (`self.LeavesXYMax`)))
  (set `self.LeavesZ` (`KismetMathLibrary.RandomFloatInRange` (`self.LeavesZMin`) (`self.LeavesZMax`)))
  (`SceneComponent.SetRelativeScale3D` (`self.Leaves`) (`KismetMathLibrary.MakeVector` (`self.LeavesX`) (`self.LeavesY`) (`self.LeavesZ`)))
  ;[1 1 1] Tune leaves Z offset
  (`SceneComponent.K2_AddRelativeLocation` (`self.Leaves`) (`KismetMathLibrary.MakeVector` 0.0 0.0 (+ (* (- (`self.LeavesZ`) 1.0) 50.0) (* (- (`self.TrunkZ`) 1.0) 100.0))) false false))

(fn `UserConstructionScript`)